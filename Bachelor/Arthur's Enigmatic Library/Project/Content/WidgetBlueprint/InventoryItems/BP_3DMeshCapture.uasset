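; 3D mesh capture actor that displays an inventory item as a static mesh the player can rotate with the mouse.
; An OnUpdateMesh event binding swaps the Item component's mesh.
; While in inventory, holding left click enables rotation: horizontal movement adds yaw, vertical movement adds both pitch and yaw.
; ResetRotation restores the world rotation saved at BeginPlay.
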(event Custom|Update%20Mesh
  (params (StaticMesh :type Static%20Mesh%20Object%20Reference))
  (Components|StaticMesh|SetStaticMesh (Variables|Default|GetItem) StaticMesh))

(event Custom|Reset%20Rotation
  (Transformation|SetWorldRotation (Variables|Default|GetItem) (Variables|Default|GetOriginalRotation) false false))

(event Collision|EventActorBeginOverlap
  (params (OtherActor :type Actor%20Object%20Reference)))

(event EventTick
  (params (DeltaSeconds :type Float%20%28single-precision%29)))

(event EventBeginPlay
  (EventDispatchers|BindEventtoOnUpdateMesh (delegate Custom|Update%20Mesh))
  (Variables|Default|SetOriginalRotation (Transformation|GetWorldRotation (Variables|Default|GetItem))))

(event Input|ActionEvents|InputActionMouseLeftclick
  (params (Key :type Key%20Structure :default "None"))
  (:Pressed
    (if (Variables|Default|GetIs%20In%20Inventory)
      (Variables|Default|SetIs%20Rotating true)))
  (:Released
    (Variables|Default|SetIs%20Rotating false)))

(event Input|AxisEvents|InputAxisMouseUp/Down
  (params (AxisValue :type Float%20%28single-precision%29))
  (bind _returnvalue (* AxisValue -5.0))
  ;[1 1 1] Rotate
  (if (Variables|Default|GetIs%20Rotating)
    (Transformation|SetWorldRotation (Variables|Default|GetItem) (Math|Rotator|CombineRotators (Transformation|GetWorldRotation (Variables|Default|GetItem)) (Math|Rotator|MakeRotator 0.0 _returnvalue _returnvalue)) false false)))

(event Input|AxisEvents|InputAxisMouseRight/Left
  (params (AxisValue :type Float%20%28single-precision%29))
  ;[1 1 1] Rotate
  (if (Variables|Default|GetIs%20Rotating)
    (Transformation|SetWorldRotation (Variables|Default|GetItem) (Math|Rotator|CombineRotators (Transformation|GetWorldRotation (Variables|Default|GetItem)) (Math|Rotator|MakeRotator 0.0 0.0 (* AxisValue -5.0))) false false)))

(fn ConstructionScript)

(fn SetUpdate?
  (params (Update? :type Boolean))
  (Variables|Default|SetUpdate? Update?))

(fn SetCurMesh
  (params (Static%20Mesh :type Static%20Mesh%20Object%20Reference))
  (Variables|Default|SetCurMesh Static%20Mesh))

(fn SetIsinInventory
  (params (Is%20In%20Inventory :type Boolean))
  (Variables|Default|SetIs%20In%20Inventory Is%20In%20Inventory))