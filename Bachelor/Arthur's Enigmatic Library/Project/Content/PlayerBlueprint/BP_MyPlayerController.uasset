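; First-person player character, despite the controller name, handling movement, mouse look, crouching, interaction and the in-game menu.
; A short camera line trace runs each tick to toggle the interact prompt, and again on key press to message InteractInterface actors with the menu's inventory.
; Crouch swaps capsule height and walk speed.
; Pause opens the menu with UI-only input but never pauses the game, as that toggle logic is disconnected.
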(event EventTick
  (params (DeltaSeconds :type Float%20%28single-precision%29))
  (CallFunction|CheckifCanInteract))

(event EventBeginPlay
  (bind _returnvalue (UserInterface|CreateWidget "/Game/PlayerBlueprint/WB_Interact.WB_Interact_C"))
  (Variables|Default|SetInteract%20UI%20Ref _returnvalue)
  (Utilities|IsValid (Variables|Default|GetIngame%20Menu%20Ref)
    (:Is%20Not%20Valid
      (bind _returnvalue_2 (UserInterface|CreateWidget "/Game/WidgetBlueprint/WB_IngameMenu.WB_IngameMenu_C" 0 (Variables|Components|GetInventory%20Component)))
      (Variables|Default|SetIngame%20Menu%20Ref _returnvalue_2))))

(event Input|ActionEvents|InputActionCrouch
  (params (Key :type Key%20Structure :default "None"))
  (:Pressed
    (CallFunction|Crouching true))
  (:Released
    (CallFunction|Crouching false)))

(event Input|ActionEvents|InputActionInteract
  (params (Key :type Key%20Structure :default "None"))
  (:Pressed
    (CallFunction|Interacting)))

(event Input|ActionEvents|InputActionPauseGame
  (params (Key :type Key%20Structure :default "None"))
  (:Pressed
    (CallFunction|Pausemenu)))

(event Input|AxisEvents|InputAxisUp/Down
  (params (AxisValue :type Float%20%28single-precision%29))
  ;[1 1 1] Movement
  (bind _fordwardvector (CallFunction|GetControlVector))
  (Pawn|Input|AddMovementInput _fordwardvector AxisValue false))

(event Input|AxisEvents|InputAxisMouseUp/Down
  (params (AxisValue :type Float%20%28single-precision%29))
  ;[1 1 1] Mouse
  (Pawn|Input|AddControllerPitchInput AxisValue))

(event Input|AxisEvents|InputAxisMouseRight/Left
  (params (AxisValue :type Float%20%28single-precision%29))
  ;[1 1 1] Mouse
  (Pawn|Input|AddControllerYawInput AxisValue))

(event Input|AxisEvents|InputAxisRight/Left
  (params (AxisValue :type Float%20%28single-precision%29))
  ;[1 1 1] Movement
  (bind _rigthvector (CallFunction|GetControlVector))
  (Pawn|Input|AddMovementInput _rigthvector AxisValue false))

(fn ConstructionScript)

(fn Pausemenu
  (bind _returnvalue (Game|GetPlayerController 0))
  ;[1 1 1] Pause Menu
  (UserInterface|Viewport|AddtoViewport (Variables|Default|GetIngame%20Menu%20Ref) 0)
  (Variables|/Script/Engine.PlayerController|SetbShowMouseCursor _returnvalue true)
  (Input|SetInputModeGameandUI _returnvalue 0 "DoNotLock" false)
  (Input|SetInputModeUIOnly _returnvalue 0 "DoNotLock"))

(fn Crouching
  (params (isPressed :type Boolean))
  (bind _capsulecomponent (Variables|Collision|GetCapsuleComponent))
  (bind _charactermovement (Variables|Character|GetCharacterMovement))
  ;[1 1 1] Crouch
  (if isPressed
    (Components|Capsule|SetCapsuleHalfHeight _capsulecomponent 7e+01 true)
    (Variables|/Script/Engine.CharacterMovementComponent|SetMaxWalkSpeed _charactermovement (Variables|Default|GetCrouchspeed))
    (else
      (Components|Capsule|SetCapsuleHalfHeight _capsulecomponent 1e+02 true)
      (Variables|/Script/Engine.CharacterMovementComponent|SetMaxWalkSpeed _charactermovement (Variables|Default|GetWalkspeed)))))

(fn Interacting
  (bind _camera (Variables|Components|GetCamera))
  (bind _returnvalue (Transformation|GetWorldLocation _camera))
  ;[1 1 1] Interact (Bool)
  (Widget|RemovefromParent (Variables|Default|GetInteract%20UI%20Ref))
  (bind _outhit (Collision|LineTraceByChannel _returnvalue (+ (* (Math|Vector|GetForwardVector (Transformation|GetWorldRotation _camera)) 1.2e+02) _returnvalue) "TraceTypeQuery1" false 0 "None"))
  (if (.bBlockingHit (Collision|BreakHitResult _outhit))
    (if (Utilities|DoesObjectImplementInterface (.HitActor (Collision|BreakHitResult _outhit)) "/Game/InventorySystem/InteractInterface.InteractInterface_C")
      (Class|InteractInterface|Interact(Message) (.HitActor (Collision|BreakHitResult _outhit)) self (Variables|/Game/WidgetBlueprint/WB_IngameMenu.WB_IngameMenu_C|GetWB_Inventory (Variables|Default|GetIngame%20Menu%20Ref)) (.HitComponent (Collision|BreakHitResult _outhit))))))

(fn GetControlVector
  (bind _returnvalue (Pawn|GetControlRotation :!class /Script/Engine.Pawn))
  (bind _yaw (Math|Rotator|BreakRotator _returnvalue))
  (bind _returnvalue_2 (Math|Rotator|MakeRotator 0.0 0.0 _yaw))
  (return (Math|Vector|GetForwardVector _returnvalue_2) (Math|Vector|GetRightVector _returnvalue_2)))

(fn CheckifCanInteract
  (bind _camera (Variables|Components|GetCamera))
  (bind _interact_ui_ref (Variables|Default|GetInteract%20UI%20Ref))
  (bind _returnvalue (Transformation|GetWorldLocation _camera))
  (bind _outhit (Collision|LineTraceByChannel _returnvalue (+ (* (Math|Vector|GetForwardVector (Transformation|GetWorldRotation _camera)) 1.2e+02) _returnvalue) "TraceTypeQuery1" false 0 "None"))
  (if (.bBlockingHit (Collision|BreakHitResult _outhit))
    (if (Utilities|DoesObjectImplementInterface (.HitActor (Collision|BreakHitResult _outhit)) "/Game/InventorySystem/InteractInterface.InteractInterface_C")
      (if (not (UserInterface|Viewport|IsinViewport _interact_ui_ref))
        (if (not (Variables|Default|GetIsInMinigame))
          (UserInterface|Viewport|AddtoViewport _interact_ui_ref 0)))
      (else
        (Widget|RemovefromParent _interact_ui_ref)))
    (else
      (Widget|RemovefromParent _interact_ui_ref))))