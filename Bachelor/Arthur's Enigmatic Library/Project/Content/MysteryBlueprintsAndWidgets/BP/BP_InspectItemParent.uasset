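; Parent Blueprint for inspectable items that the player can bring up in front of the camera to examine.
; Interact stores the item's transform, flags the player as in a minigame, and hands input from player to item.
; Zoom actions move it along the camera's forward vector within a clamped range, while left-click dragging rotates it.
; Pressing Interact again restores the transform, player input and minigame flag.
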(event EventInteract
  (params (Player :type BP%20My%20Player%20Controller%20Object%20Reference) (Inventory :type WB%20Inventory%20Object%20Reference) (Hit%20Component :type Actor%20Component%20Object%20Reference))
  (bind _returnvalue (Game|GetPlayerController 0))
  (bind _returnvalue_2 (Game|GetPlayerCameraManager 0))
  (bind _defaultsceneroot (Variables|Default|GetDefaultSceneRoot))
  ;[1 1 1] Interact and Endinteract
  (Variables|/Game/PlayerBlueprint/BP_MyPlayerController.BP_MyPlayerController_C|SetIsInMinigame Player true)
  (bind _output_get (Variables|Default|SetStartPosition (Transformation|GetWorldLocation _defaultsceneroot)))
  (bind _output_get_2 (Variables|Default|SetStartRotation (Transformation|GetWorldRotation _defaultsceneroot)))
  (Input|DisableInput Player _returnvalue)
  (Input|EnableInput self _returnvalue)
  (Transformation|SetActorLocation (+ (Camera|GetCameraLocation _returnvalue_2) (* (Math|Vector|GetForwardVector (Camera|GetCameraRotation _returnvalue_2)) 2e+01)) false false))

(event Input|ActionEvents|InputActionInteract
  (params (Key :type Key%20Structure :default "None"))
  (bind _returnvalue (Game|GetPlayerController 0))
  ;[1 1 1] Interact and Endinteract
  (:Pressed
    (Input|DisableInput _returnvalue)
    (Input|EnableInput (stale EventInteract Player) _returnvalue)
    (Transformation|SetActorLocation (stale EventInteract _output_get) false false)
    (Transformation|SetActorRotation (stale EventInteract _output_get_2))
    (Variables|/Game/PlayerBlueprint/BP_MyPlayerController.BP_MyPlayerController_C|SetIsInMinigame (stale EventInteract Player) false)))

(event Input|ActionEvents|InputActionMouseLeftclick
  (params (Key :type Key%20Structure :default "None"))
  (:Pressed
    (Variables|Default|SetIsRotating true))
  (:Released
    (Variables|Default|SetIsRotating false)))

(event Input|ActionEvents|InputActionZoomUP
  (params (Key :type Key%20Structure :default "None"))
  (bind _returnvalue (Game|GetPlayerCameraManager 0))
  (:Pressed
    (bind _output_get (Variables|Default|SetZoomlevel (Math|Integer|Clamp(Integer) (- (Variables|Default|GetZoomlevel) 1) 15 40)))
    (if (> _output_get 15)
      (Transformation|SetActorLocation (+ (Camera|GetCameraLocation _returnvalue) (* (Math|Vector|GetForwardVector (Camera|GetCameraRotation _returnvalue)) (Math|Conversions|ToFloat(Integer) (Variables|Default|GetZoomlevel)))) false false))))

(event Input|ActionEvents|InputActionZoomDOWN
  (params (Key :type Key%20Structure :default "None"))
  (bind _returnvalue (Game|GetPlayerCameraManager 0))
  (:Pressed
    (bind _output_get (Variables|Default|SetZoomlevel (Math|Integer|Clamp(Integer) (+ (Variables|Default|GetZoomlevel) 1) 15 40)))
    (if (< _output_get 40)
      (Transformation|SetActorLocation (+ (Camera|GetCameraLocation _returnvalue) (* (Math|Vector|GetForwardVector (Camera|GetCameraRotation _returnvalue)) (Math|Conversions|ToFloat(Integer) (Variables|Default|GetZoomlevel)))) false false))))

(event Input|AxisEvents|InputAxisMouseUp/Down
  (params (AxisValue :type Float%20%28single-precision%29))
  (bind _returnvalue (* AxisValue -5.0))
  ;[1 1 1] Rotate
  (if (Variables|Default|GetIsRotating)
    (Transformation|SetActorRotation (Math|Rotator|CombineRotators (Transformation|GetActorRotation) (Math|Rotator|MakeRotator 0.0 _returnvalue _returnvalue)))))

(event Input|AxisEvents|InputAxisMouseRight/Left
  (params (AxisValue :type Float%20%28single-precision%29))
  ;[1 1 1] Rotate
  (if (Variables|Default|GetIsRotating)
    (Transformation|SetActorRotation (Math|Rotator|CombineRotators (Transformation|GetActorRotation) (Math|Rotator|MakeRotator 0.0 0.0 (* AxisValue -5.0))))))

(fn ConstructionScript)