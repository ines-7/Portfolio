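; Possessable four-dial combination lock puzzle that the player enters through Interact, with a camera blend and UI widget.
; Minigame inputs rotate the highlighted dial in 36-degree steps, track its digit with wraparound and cycle between dials.
; Enter checks all four digits, then blends to ChangeCam and calls Solved on SolvedObject through SolvedInterface.
; Pressing Interact again restores the player's view and possession; a similar exit sequence is left unwired.
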(event EventInteract
  (params (Player :type BP%20My%20Player%20Controller%20Object%20Reference) (Inventory :type WB%20Inventory%20Object%20Reference) (Hit%20Component :type Actor%20Component%20Object%20Reference))
  (bind _returnvalue (Game|GetPlayerController 0))
  (bind _self self)
  ;[1 1 1] Start To Interact with Camera Switch
  (Variables|/Game/PlayerBlueprint/BP_MyPlayerController.BP_MyPlayerController_C|SetIsInMinigame Player true)
  (Utilities|IsValid (Variables|Default|GetCombinationLockWB)
    (:Is%20Valid
      _)
    (:Is%20Not%20Valid
      (bind _returnvalue_2 (UserInterface|CreateWidget "/Game/MysteryBlueprintsAndWidgets/WB/WB_Combinationlock.WB_Combinationlock_C"))
      (Variables|Default|SetCombinationLockWB _returnvalue_2)))
  (bind _output_get (Variables|Default|SetPlayer Player))
  (Game|Player|SetViewTargetwithBlend _returnvalue _self 0.4 "VTBlend_EaseIn" 0.4 true)
  (Utilities|FlowControl|Delay 0.4)
  (Pawn|Possess _returnvalue _self)
  (bind _output_get_2 (Variables|Default|SetCurrentCode (Variables|Default|GetCode01)))
  (Rendering|Material|SetScalarParameterValueonMaterials _output_get_2 "isHighlighted" 1.0)
  (UserInterface|Viewport|AddtoViewport (Variables|Default|GetCombinationLockWB) 0))

(event Input|ActionEvents|InputActionInteract
  (params (Key :type Key%20Structure :default "None"))
  (bind _returnvalue (Game|GetPlayerController 0))
  ;[1 1 1] Start To Interact with Camera Switch
  (:Pressed
    (Widget|RemovefromParent (Variables|Default|GetCombinationLockWB))
    (Game|Player|SetViewTargetwithBlend _returnvalue (stale EventInteract _output_get) 0.4 "VTBlend_EaseOut" 0.4 false)
    (Utilities|FlowControl|Delay 0.5)
    (Pawn|Possess _returnvalue (stale EventInteract _output_get))
    (Variables|/Game/PlayerBlueprint/BP_MyPlayerController.BP_MyPlayerController_C|SetIsInMinigame (Variables|Default|GetPlayer) false)
    (Rendering|Material|SetScalarParameterValueonMaterials (Variables|Default|GetCurrentCode) "isHighlighted" 0.0)))

(event Input|ActionEvents|InputActionMinigameDOWN
  (params (Key :type Key%20Structure :default "None"))
  (:Pressed
    (if (not (Variables|Default|GetisFinished))
      (if (not (Variables|Default|GetisInMove))
        (Variables|Default|SetisInMove true)
        (Transformation|AddRelativeRotation (Variables|Default|GetCurrentCode) "0, 0,-36.000000" false false)
        (Variables|Default|SetisInMove false)
        (CallFunction|CountDown)))))

(event Input|ActionEvents|InputActionMinigameUP
  (params (Key :type Key%20Structure :default "None"))
  (:Pressed
    (if (not (Variables|Default|GetisFinished))
      (if (not (Variables|Default|GetisInMove))
        (Variables|Default|SetisInMove true)
        (Transformation|AddRelativeRotation (Variables|Default|GetCurrentCode) "0.000000, 0,36.000000" false false)
        (Variables|Default|SetisInMove false)
        (CallFunction|CountUp)))))

(event Input|ActionEvents|InputActionMinigameENTER
  (params (Key :type Key%20Structure :default "None"))
  (bind _solvedobject (Variables|Default|GetSolvedObject))
  (:Pressed
    (if (== (Variables|Default|GetCode1) (Variables|Default|GetCode1Solution))
      (if (== (Variables|Default|GetCode2) (Variables|Default|GetCode2Solution))
        (if (== (Variables|Default|GetCode3) (Variables|Default|GetCode3Solution))
          (if (== (Variables|Default|GetCode4) (Variables|Default|GetCode4Solution))
            (Game|Player|SetViewTargetwithBlend (Game|GetPlayerController 0) (Variables|Default|GetChangeCam) 1.0 "VTBlend_Linear" 0.0 false)
            (Utilities|FlowControl|Delay 1.0)
            (if (Utilities|IsValid (Utilities|ToObject(Interface) _solvedobject))
              (if (Utilities|DoesObjectImplementInterface (Utilities|ToObject(Interface) _solvedobject) "/Game/MysteryBlueprintsAndWidgets/BP/SolvedInterface.SolvedInterface_C")
                (Default|Solved _solvedobject (Variables|Default|GetPlayer))))))))))

(event Input|ActionEvents|InputActionMinigameNext
  (params (Key :type Key%20Structure :default "None"))
  (:Pressed
    (CallFunction|Change)))

(fn ConstructionScript)

(fn Change
  (if (not (Variables|Default|GetisInMove))
    (Rendering|Material|SetScalarParameterValueonMaterials (Variables|Default|GetCurrentCode) "isHighlighted" 0.0)
    (bind _result (Math|Integer|IncrementInt (Variables|Default|GetWhichCode))
      (:%20%20
        (switch int _result
          (:0
            (bind _output_get (Variables|Default|SetCurrentCode (Variables|Default|GetCode01) :!label _label)))
          (:1
            (bind _output_get_2 (Variables|Default|SetCurrentCode (Variables|Default|GetCode02))))
          (:2
            (bind _output_get_3 (Variables|Default|SetCurrentCode (Variables|Default|GetCode03))))
          (:3
            (bind _output_get_4 (Variables|Default|SetCurrentCode (Variables|Default|GetCode04))))
          (:4
            (Variables|Default|SetWhichCode 0)
            (goto _label)))
        (Rendering|Material|SetScalarParameterValueonMaterials _output_get "isHighlighted" 1.0)))))

(fn CountUp
  (switch int (Variables|Default|GetWhichCode)
    (:0
      (if (<= (Variables|Default|GetCode1) 8)
        (bind _result (Math|Integer|IncrementInt (Variables|Default|GetCode1))
          (:%20%20
            (Variables|Default|SetCode1 _result)))
        (else
          (Variables|Default|SetCode1 0))))
    (:1
      (if (<= (Variables|Default|GetCode2) 8)
        (bind _result_2 (Math|Integer|IncrementInt (Variables|Default|GetCode2))
          (:%20%20
            (Variables|Default|SetCode2 _result_2)))
        (else
          (Variables|Default|SetCode2 0))))
    (:2
      (if (<= (Variables|Default|GetCode3) 8)
        (bind _result_3 (Math|Integer|IncrementInt (Variables|Default|GetCode3))
          (:%20%20
            (Variables|Default|SetCode3 _result_3)))
        (else
          (Variables|Default|SetCode3 0))))
    (:3
      (if (<= (Variables|Default|GetCode4) 8)
        (bind _result_4 (Math|Integer|IncrementInt (Variables|Default|GetCode4))
          (:%20%20
            (Variables|Default|SetCode4 _result_4)))
        (else
          (Variables|Default|SetCode4 0))))
    (:4
      (Variables|Default|SetWhichCode 0))))

(fn CountDown
  (switch int (Variables|Default|GetWhichCode)
    (:0
      (if (>= (Variables|Default|GetCode1) 1)
        (bind _result (Math|Integer|DecrementInt (Variables|Default|GetCode1))
          (:%20%20
            (Variables|Default|SetCode1 _result)))
        (else
          (Variables|Default|SetCode1 9))))
    (:1
      (if (>= (Variables|Default|GetCode2) 1)
        (bind _result_2 (Math|Integer|DecrementInt (Variables|Default|GetCode2))
          (:%20%20
            (Variables|Default|SetCode2 _result_2)))
        (else
          (Variables|Default|SetCode2 9))))
    (:2
      (if (>= (Variables|Default|GetCode3) 1)
        (bind _result_3 (Math|Integer|DecrementInt (Variables|Default|GetCode3))
          (:%20%20
            (Variables|Default|SetCode3 _result_3)))
        (else
          (Variables|Default|SetCode3 9))))
    (:3
      (if (>= (Variables|Default|GetCode4) 1)
        (bind _result_4 (Math|Integer|DecrementInt (Variables|Default|GetCode4))
          (:%20%20
            (Variables|Default|SetCode4 _result_4)))
        (else
          (Variables|Default|SetCode4 9))))))