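; Possessable Sudoku puzzle that serves as a minigame, taking over camera and control from the player on interact.
; The Interact input then alternately shows a reused WB_Sodoku widget with mouse cursor, or removes it and blends back to repossess the player.
; Tick polls the widget's Finished flag, then toggles the unsolved and solved book meshes.
; Once finished, the input only exits back to the player.
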(event EventTick
  (params (DeltaSeconds :type Float%20%28single-precision%29))
  ;[1 1 1] Finishing
  (if (not (Variables|Default|GetisFinished))
    (if (Variables|Default|GetWidgetExist)
      (if (Variables|/Game/MysteryBlueprintsAndWidgets/WB/WB_Sodoku.WB_Sodoku_C|GetFinished (Variables|Default|GetSodokuWidget))
        (Variables|Default|SetisFinished true)
        (Rendering|ToggleVisibility (Variables|Default|GetSM_SudokuBook_unsolved) false)))))

(event EventInteract
  (params (Player :type BP%20My%20Player%20Controller%20Object%20Reference))
  (bind _returnvalue (Game|GetPlayerController 0))
  (bind _self self)
  ;[1 1 1] Start To Interact with Camera Switch
  (Variables|/Game/PlayerBlueprint/BP_MyPlayerController.BP_MyPlayerController_C|SetIsInMinigame Player true)
  (bind _output_get (Variables|Default|SetPlayer Player))
  (Game|Player|SetViewTargetwithBlend _returnvalue _self 0.4 "VTBlend_EaseIn" 0.4 true)
  (Utilities|FlowControl|Delay 0.4)
  (Pawn|Possess _returnvalue _self))

(event Input|ActionEvents|InputActionInteract
  (params (Key :type Key%20Structure)))

(event Input|ActionEvents|InputActionInteract
  (params (Key :type Key%20Structure))
  (bind _returnvalue (Game|GetPlayerController 0))
  ;[1 1 1] Start To Interact with Camera Switch
  (:Pressed
    (if (Variables|Default|GetisFinished)
      (Widget|RemovefromParent (stale _returnvalue_2) :!label _label)
      (Game|Player|SetViewTargetwithBlend _returnvalue (stale EventInteract _output_get) 0.4 "VTBlend_EaseOut" 0.4 false)
      (Utilities|FlowControl|Delay 0.5)
      (Pawn|Possess _returnvalue (stale EventInteract _output_get))
      (Variables|/Game/PlayerBlueprint/BP_MyPlayerController.BP_MyPlayerController_C|SetIsInMinigame (Variables|Default|GetPlayer) false)
      (Variables|/Script/Engine.PlayerController|SetbShowMouseCursor _returnvalue false)
      (Input|SetInputModeGameOnly _returnvalue)
      (else
        (Utilities|FlowControl|FlipFlop
          (:A
            (if (Variables|Default|GetWidgetExist)
              _
              (else
                (bind _returnvalue_2 (UserInterface|CreateWidget "/Game/MysteryBlueprintsAndWidgets/WB/WB_Sodoku.WB_Sodoku_C"))
                (Variables|Default|SetSodokuWidget _returnvalue_2)))
            (UserInterface|Viewport|AddtoViewport _returnvalue_2 0)
            (Variables|Default|SetWidgetExist true)
            (Variables|/Script/Engine.PlayerController|SetbShowMouseCursor _returnvalue true)
            (Input|SetInputModeGameandUI _returnvalue 0 "DoNotLock" true))
          (:B
            (goto _label)))))))

(fn ConstructionScript)