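; BP_Casket is an interactable puzzle casket that accepts three puzzle pieces from the interacting player.
; Interact reveals each missing piece's component when the player holds that piece and records it as placed.
; CheckIfFinished hides BoxHead once all three are placed, but runs only while piece three was still missing at that step.
; IsFinished gates interaction but is never set here.
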(event EventBeginPlay)

(event Collision|EventActorBeginOverlap
  (params (OtherActor :type Actor%20Object%20Reference)))

(event EventTick
  (params (DeltaSeconds :type Float%20%28single-precision%29)))

(event EventInteract
  (params (Player :type BP%20My%20Player%20Controller%20Object%20Reference) (Inventory :type WB%20Inventory%20Object%20Reference) (Hit%20Component :type Actor%20Component%20Object%20Reference))
  (Variables|Default|SetPlayer Player)
  (if (not (Variables|Default|GetisFinished))
    (if (Variables|Default|GetHasPuzzle1)
      _
      (elif (Variables|/Game/PlayerBlueprint/BP_MyPlayerController.BP_MyPlayerController_C|GetHasPuzzlePiece1 (Variables|Default|GetPlayer))
        (Rendering|SetVisibility (Variables|Default|GetPuzzle1) true false)
        (Variables|Default|SetHasPuzzle1 true)))
    (if (Variables|Default|GetHasPuzzle2)
      _
      (elif (Variables|/Game/PlayerBlueprint/BP_MyPlayerController.BP_MyPlayerController_C|GetHasPuzzlePiece2 (Variables|Default|GetPlayer))
        (Rendering|SetVisibility (Variables|Default|GetPuzzle2) true false)
        (Variables|Default|SetHasPuzzle2 true)))
    (if (not (Variables|Default|GetHasPuzzle3))
      (if (Variables|/Game/PlayerBlueprint/BP_MyPlayerController.BP_MyPlayerController_C|GetHasPuzzlePiece3 (Variables|Default|GetPlayer))
        (Rendering|SetVisibility (Variables|Default|GetPuzzle3) true false)
        (Variables|Default|SetHasPuzzle3 true))
      (CallFunction|CheckifFinished))))

(fn ConstructionScript)

(fn CheckifFinished
  (if (Variables|Default|GetHasPuzzle1)
    (if (Variables|Default|GetHasPuzzle2)
      (if (Variables|Default|GetHasPuzzle3)
        (Rendering|SetVisibility (Variables|Default|GetBoxHead) false false)))))