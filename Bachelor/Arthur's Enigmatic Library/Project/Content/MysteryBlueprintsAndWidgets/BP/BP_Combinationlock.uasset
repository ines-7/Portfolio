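; BP_Combinationlock is a possessable four-dial combination lock minigame; the file shows no solution check.
; Interact blends the camera to the lock, possesses it, highlights the first dial and shows its widget.
; Next input cycles the highlighted dial through a material parameter, while Up and Down spin it via timelines, guarded against overlapping moves.
; Pressing Interact again removes the widget, blends back to the player and repossesses them.
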(event EventInteract
  (params (Player :type BP%20My%20Player%20Controller%20Object%20Reference))
  (bind _returnvalue (Game|GetPlayerController 0))
  (bind _self self)
  ;[1 1 1] Start To Interact with Camera Switch
  (Utilities|IsValid (Variables|Default|GetCombinationLockWB)
    (:Is%20Valid
      _)
    (:Is%20Not%20Valid
      (bind _returnvalue_2 (UserInterface|CreateWidget "/Game/MysteryBlueprintsAndWidgets/WB/WB_Combinationlock.WB_Combinationlock_C"))
      (Variables|Default|SetCombinationLockWB _returnvalue_2)))
  (bind _output_get (Variables|Default|SetPlayer Player))
  (Game|Player|SetViewTargetwithBlend _returnvalue _self 0.4 "VTBlend_EaseIn" 0.4 true)
  (Utilities|FlowControl|Delay 0.4)
  (Pawn|Possess _returnvalue _self)
  (bind _output_get_2 (Variables|Default|SetCurrentCode (Variables|Default|GetCode1)))
  (Rendering|Material|SetScalarParameterValueonMaterials _output_get_2 "isHighlighted" 1.0)
  (UserInterface|Viewport|AddtoViewport (Variables|Default|GetCombinationLockWB) 0))

(event Input|ActionEvents|InputActionInteract
  (params (Key :type Key%20Structure))
  (bind _returnvalue (Game|GetPlayerController 0))
  ;[1 1 1] Start To Interact with Camera Switch
  (:Pressed
    (Widget|RemovefromParent (Variables|Default|GetCombinationLockWB))
    (Game|Player|SetViewTargetwithBlend _returnvalue (stale EventInteract _output_get) 0.4 "VTBlend_EaseOut" 0.4 false)
    (Utilities|FlowControl|Delay 0.5)
    (Pawn|Possess _returnvalue (stale EventInteract _output_get))
    (Variables|/Game/PlayerBlueprint/BP_MyPlayerController.BP_MyPlayerController_C|SetIsInMinigame (Variables|Default|GetPlayer) false)
    (Rendering|Material|SetScalarParameterValueonMaterials (Variables|Default|GetCurrentCode) "isHighlighted" 0.0)))

(event Input|ActionEvents|InputActionMinigameDOWN
  (params (Key :type Key%20Structure))
  (:Pressed
    (if (not (Variables|Default|GetisInMove))
      (bind _newtrack_0 (Timeline|Timeline_1 PlayFromStart)
        (:Update
          (Variables|Default|SetisInMove true)
          (Transformation|AddLocalRotation (Variables|Default|GetCurrentCode) (Math|Rotator|MakeRotator 0.0 0.0 (* _newtrack_0 -1.0)) false false))
        (:Finished
          (Variables|Default|SetisInMove false))))))

(event Input|ActionEvents|InputActionMinigameUP
  (params (Key :type Key%20Structure))
  (:Pressed
    (if (not (Variables|Default|GetisInMove))
      (bind _newtrack_0 (Timeline|Timeline_0 PlayFromStart)
        (:Update
          (Variables|Default|SetisInMove true)
          (Transformation|AddLocalRotation (Variables|Default|GetCurrentCode) (Math|Rotator|MakeRotator 0.0 0.0 _newtrack_0) false false))
        (:Finished
          (Variables|Default|SetisInMove false))))))

(event Input|ActionEvents|InputActionMinigameNext
  (params (Key :type Key%20Structure))
  (:Pressed
    (CallFunction|Change)))

(fn ConstructionScript)

(fn Change
  (if (not (Variables|Default|GetisInMove))
    (Rendering|Material|SetScalarParameterValueonMaterials (Variables|Default|GetCurrentCode) "isHighlighted" 0.0)
    (bind _result (Math|Integer|IncrementInt (Variables|Default|GetWhichCode))
      (:%20%20
        (switch int _result
          (:0
            (bind _output_get (Variables|Default|SetCurrentCode (Variables|Default|GetCode1) :!label _label)))
          (:1
            (bind _output_get_2 (Variables|Default|SetCurrentCode (Variables|Default|GetCode2))))
          (:2
            (bind _output_get_3 (Variables|Default|SetCurrentCode (Variables|Default|GetCode3))))
          (:3
            (bind _output_get_4 (Variables|Default|SetCurrentCode (Variables|Default|GetCode4))))
          (:4
            (Variables|Default|SetWhichCode 0)
            (goto _label)))
        (Rendering|Material|SetScalarParameterValueonMaterials _output_get "isHighlighted" 1.0)))))